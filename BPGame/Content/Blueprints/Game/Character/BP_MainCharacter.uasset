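; Player character Blueprint handling Enhanced Input movement, look and jump, weapon pickup, attacking and death.
; Attack input activates a Gameplay Ability System ability, whose start and end events lock and restore movement unless the Dead tag is present.
; A collected weapon attaches to the hand socket and receives attack-check start/end events for its hit window.
; GAS death sets CharacterState, plays the death montage and disables collision; older montage-attack and damage logic remains unwired.
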(event `self.ReceiveBeginPlay`)

(event `self.OnGasDeath`
  (`self.OnPlayerDied`))

(event `OnPlayerDied`
  (set `self.CharacterState` "NewEnumerator2")
  (`self.PlayAnimMontage` "/Game/Blueprints/Game/Animation/AM_Dead.AM_Dead")
  (`self.SetActorEnableCollision` false)
  (set `self.Tags` (`|MakeArray` "None" :!type "Name")))

(event `EnhancedInput|/Game/Blueprints/Input/IA_Jump`
  (params (ActionValue :type Boolean) (ElapsedSeconds :type "Float (double-precision)") (TriggeredSeconds :type "Float (double-precision)") (InputAction :type "InputAction Object Reference" :default "/Game/Blueprints/Input/IA_Jump.IA_Jump"))
  ; 점프 처리
  (:`Triggered`
    (`self.Jump`))
  (:`Canceled`
    (`self.StopJumping`)))

(event `EnhancedInput|/Game/Blueprints/Input/IA_Move`
  (params (ActionValue :type "Vector2D Structure") (ElapsedSeconds :type "Float (double-precision)") (TriggeredSeconds :type "Float (double-precision)") (InputAction :type "InputAction Object Reference" :default "/Game/Blueprints/Input/IA_Move.IA_Move"))
  (bind (_returnvalue_roll _returnvalue_pitch _returnvalue_yaw) (`KismetMathLibrary.BreakRotator` (`self.GetControlRotation`)))
  ;[0.1413 0.04572 0.15 0.5] 캐릭터 이동
  (:`Triggered`
    (switch `/Game/Blueprints/Game/Character/E_CharacterState` (`self.CharacterState`)
      (:`NewEnumerator0`
        (`self.AddMovementInput` (+ (* ActionValue_X (`KismetMathLibrary.GetRightVector` (`KismetMathLibrary.MakeRotator` 0.0 0.0 _returnvalue_yaw))) (* ActionValue_Y (`KismetMathLibrary.GetForwardVector` (`KismetMathLibrary.MakeRotator` 0.0 0.0 _returnvalue_yaw)))))))))

(event `EnhancedInput|/Game/Blueprints/Input/IA_Look`
  (params (ActionValue :type "Vector2D Structure") (ElapsedSeconds :type "Float (double-precision)") (TriggeredSeconds :type "Float (double-precision)") (InputAction :type "InputAction Object Reference" :default "/Game/Blueprints/Input/IA_Look.IA_Look"))
  ;[0.15 0.1141 0.02538 0.5] 카메라 회전
  (:`Triggered`
    (`self.AddControllerYawInput` ActionValue_X)
    (`self.AddControllerPitchInput` (* ActionValue_Y -1.0))))

(event `EnhancedInput|/Game/Blueprints/Input/IA_Attack`
  (params (ActionValue :type Boolean) (ElapsedSeconds :type "Float (double-precision)") (TriggeredSeconds :type "Float (double-precision)") (InputAction :type "InputAction Object Reference" :default "/Game/Blueprints/Input/IA_Attack.IA_Attack"))
  ; 공격 입력
  (:`Triggered`
    (`self.TryActivateAttackAbility`)))

(event `OnAttackEnd`
  ;[0.07111 0.1113 0.15 0.5] 공격 종료 처리
  (set `self.CharacterState` "NewEnumerator0"))

(event `self.OnGasAttackStarted`
  (`MovementComponent.StopMovementImmediately` (`self.CharacterMovement`))
  (`CharacterMovementComponent.DisableMovement` (`self.CharacterMovement`)))

(event `self.OnGasAttackEnded`
  (params (bWasCancelled :type Boolean))
  (if (not (`GameplayTagAssetInterface.HasMatchingGameplayTag` (`self.AbilitySystemComponent`) (struct :`TagName` "State.Dead")))
    (`CharacterMovementComponent.SetMovementMode` (`self.CharacterMovement`) "MOVE_Walking" 0)))

(event `OnAttack`
  ;[0.05414 0.07593 0.15 0.5] 공격 시작 처리
)

(event `OnWeaponCollected`
  (params (Weapon :type "/Game/Blueprints/Game/Actor/BP_Weapon Object Reference"))
  ;[0.05146 0.15 0.06155 0.5] 무기 획득 처리
  (bind _output_get (set `self.Weapon` Weapon))
  (`self.K2_AttachToComponent` _output_get (`self.Mesh`) "WeaponPosition" "SnapToTarget" "SnapToTarget" "SnapToTarget" true)
  ;[0.15 0.1345 0.01365 0.5] 이벤트 구독 처리
  (add `self.AttackCheckStart` (delegate `OnAttackCheckStart`)) ; 이 이벤트에 다른 이벤트를 연결
  (add `self.AttackCheckEnd` (delegate `OnAttackCheckEnd`)))

(event `OnAttackCheckStart`
  ;[0.15 0.1345 0.01365 0.5] 이벤트 구독 처리
  (`/Game/Blueprints/Game/Actor/BP_Weapon.OnAttackCheckStart` (`self.Weapon`)))

(event `OnAttackCheckEnd`
  ;[0.15 0.1345 0.01365 0.5] 이벤트 구독 처리
  (`/Game/Blueprints/Game/Actor/BP_Weapon.OnAttackCheckEnd` (`self.Weapon`)))

(event `self.ReceiveAnyDamage`
  (params (Damage :type "Float (single-precision)") (DamageType :type "DamageType Object Reference") (InstigatedBy :type "Controller Object Reference") (DamageCauser :type "Actor Object Reference")))

(fn `UserConstructionScript`)