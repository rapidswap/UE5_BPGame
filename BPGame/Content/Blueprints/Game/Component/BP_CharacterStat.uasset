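; BP_CharacterStat is a character stat component that tracks current HP.
; On BeginPlay it sets CurrentHp from MaxHp in its Data reference, if that is valid.
; ReceiveDamage subtracts damage, clamps HP at zero and calls OnHpZero whenever the result is zero, so other logic can react to depleted health.
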(event `self.ReceiveBeginPlay`
  ;[1 0.05391 0 0.5] 시작하면 데이터에 설정된 HP로 세팅
  (bind _data (`self.Data`)
    (:`then`
      (set `self.CurrentHp` (`/Game/Blueprints/Game/Data/BP_CharacterData.MaxHp` _data)))
    (:`else`)))

(event `ReceiveDamage`
  (params (Damage :type "Float (double-precision)"))
  ;[0.9708 1 0 0.5] 대미지 처리 및 HpZero 이벤트 발행
  (bind _output_get (set `self.CurrentHp` (`KismetMathLibrary.FMax` (- (`self.CurrentHp`) Damage))))
  (if (== _output_get 0.0)
    (`self.OnHpZero`)))