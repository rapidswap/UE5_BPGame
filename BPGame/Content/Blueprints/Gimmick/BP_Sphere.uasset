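; BP_Sphere is a gimmick that launches a Player-tagged Character when it begins overlapping the actor.
; It adds a velocity-change impulse to the character's movement along the Arrow component's forward vector, scaled by PushPower.
; Each launch also restarts the TurnOn timeline, which drives the Alpha parameter of a dynamic M_Sphere material created on BeginPlay, giving visual feedback.
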(event `self.ReceiveBeginPlay`
  (bind _returnvalue (`PrimitiveComponent.CreateDynamicMaterialInstance` (`self.Sphere`) 0 "/Game/Meterial/M_Sphere.M_Sphere" "None"))
  (set `self.MaterialInstance` _returnvalue))

(event `self.ReceiveActorBeginOverlap`
  (params (OtherActor :type "Actor Object Reference"))
  (if (`self.ActorHasTag` OtherActor "Player")
    (bind _ascharacter (cast `Character` OtherActor))
    (`CharacterMovementComponent.AddImpulse` (`Character.CharacterMovement` _ascharacter) (* (`SceneComponent.GetForwardVector` (`self.Arrow`)) (`self.PushPower`)) true)
    (bind (_direction _alpha) (`Timeline|Turn On` :!via `PlayFromStart`)
      (:`Update`
        (`MaterialInstanceDynamic.SetScalarParameterValue` (`self.MaterialInstance`) "Alpha" _alpha)))))

(fn `UserConstructionScript`)