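; BP_Weapon is a pickup weapon actor that the player collects and then uses to deal damage.
; Overlapping its Box with a Player-tagged BP_MainCharacter calls OnWeaponCollected on that character and disables the pickup collision.
; WeaponCollision starts disabled and is toggled to query-only by attack check start and end events.
; While it is enabled, any overlapping actor receives ApplyDamage with the weapon's Damage, instigated by player controller 0.
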(event `OnAttackCheckStart`
  (`PrimitiveComponent.SetCollisionEnabled` (`self.WeaponCollision`) "QueryOnly"))

(event `self.ReceiveBeginPlay`
  ; 시작하면 무기 콜리전 끄기
  (`PrimitiveComponent.SetCollisionEnabled` (`self.WeaponCollision`) "NoCollision"))

(event `OnAttackCheckEnd`
  (`PrimitiveComponent.SetCollisionEnabled` (`self.WeaponCollision`) "NoCollision"))

(event `self.Box.OnComponentBeginOverlap`
  (params (OverlappedComponent :type "PrimitiveComponent Object Reference") (OtherActor :type "Actor Object Reference") (OtherComp :type "PrimitiveComponent Object Reference") (OtherBodyIndex :type Integer) (bFromSweep :type Boolean) (SweepResult :type "HitResult Structure (by ref)"))
  ;[0.15 0 0.01071 0.5] 무기 획득 처리
  (if (`self.ActorHasTag` OtherActor "Player")
    (bind _asbp_main_character (cast `/Game/Blueprints/Game/Character/BP_MainCharacter` OtherActor))
    (`/Game/Blueprints/Game/Character/BP_MainCharacter.OnWeaponCollected` _asbp_main_character self)
    (`PrimitiveComponent.SetCollisionEnabled` (`self.Box`) "NoCollision")))

(event `self.WeaponCollision.OnComponentBeginOverlap`
  (params (OverlappedComponent :type "PrimitiveComponent Object Reference") (OtherActor :type "Actor Object Reference") (OtherComp :type "PrimitiveComponent Object Reference") (OtherBodyIndex :type Integer) (bFromSweep :type Boolean) (SweepResult :type "HitResult Structure (by ref)"))
  ;[0.15 0.00489 0 0.5] 무기 콜리전 충돌 처리
  ; 데미지 전달
  (`GameplayStatics.ApplyDamage` OtherActor (`self.Damage`) (`GameplayStatics.GetPlayerController` 0) self))

(fn `UserConstructionScript`)