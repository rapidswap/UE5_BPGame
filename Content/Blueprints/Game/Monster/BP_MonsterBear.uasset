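; BP_MonsterBear is an AI bear monster that detects and chases the player, deals melee damage and can be killed.
; Pawn sensing passes the player to the Blackboard, and SetState syncs Locomotion, Chase, Attack or Dead with movement speed.
; An attack collider, toggled by check start/end events, applies stat-based damage on overlap.
; Hits flash a dynamic material via timeline and reduce MonsterStat HP, whose zero event stops AI, plays death and destroys the actor.
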(event `self.ReceiveBeginPlay`
  ;[0.0221 0.15 0.13 0.5] 시작시 공격 콜리전 끄기
  (`PrimitiveComponent.SetCollisionEnabled` (`self.AttackCollision`) "NoCollision")
  ; 머터리얼 인스턴스 생성 (피격 효과를 위해)
  (bind _returnvalue (`PrimitiveComponent.CreateDynamicMaterialInstance` (`self.Mesh`) 0 "/Game/InfinityBladeAdversaries/Enemy/Enemy_Bear/Materials/M_Bear_Stone_Inst.M_Bear_Stone_Inst" "None"))
  (set `self.MaterialInstance` _returnvalue)
  ; 죽음 등록 및 처리
  (add `/Game/Blueprints/Game/Component/BP_MonsterStat.OnHpZero` (`self.MonsterStat`) (delegate `MosterDied`)))

(event `MosterDied`
  (bind _braincomponent (`AIController.BrainComponent` (`AIBlueprintHelperLibrary.GetAIController` self)))
  ; 죽음 등록 및 처리
  (`self.SetActorEnableCollision` false) ; 액터의 모든 콜리전 끄기
  (`self.PlayAnimMontage` "/Game/Blueprints/Game/Monster/Animation/AM_MonsterDead.AM_MonsterDead") ; 죽는 모션 재생
  ;;[1 0.1979 0.1979 0.5] AI 중지 처리
  (`BrainComponent.StopLogic` _braincomponent "")
  (message `NavMovementInterface.StopMovementKeepPathing` _braincomponent)
  (`self.SetState` "NewEnumerator3")
  (`KismetSystemLibrary.Delay` 2.0)
  (`self.K2_DestroyActor`))

(event `self.ReceiveAnyDamage`
  (params (Damage :type "Float (single-precision)") (DamageType :type "DamageType Object Reference") (InstigatedBy :type "Controller Object Reference") (DamageCauser :type "Actor Object Reference"))
  ;[0.03237 0.15 0.03326 0.5] 몬스터 데미지 처리
  (`KismetSystemLibrary.PrintString` "Hello")
  (`self.PlayDamageEffect`)
  (`/Game/Blueprints/Game/Component/BP_MonsterStat.ReceiveDamage` (`self.MonsterStat`) Damage))

(event `PlayDamageEffect`
  ;[1 0 0.004859 0.5] 피격 효과 재생 (머터리얼 활용)
  (bind (_direction _alpha) (`Timeline|DamageEffect` :!via `PlayFromStart`)
    (:`Update`
      (bind _materialinstance (`self.MaterialInstance`)
        (:`then`
          (`MaterialInstanceDynamic.SetScalarParameterValue` _materialinstance "DamageFactor" _alpha))
        (:`else`)))
    (:`Finished`
      (bind _materialinstance_2 (`self.MaterialInstance`)
        (:`then`
          (`MaterialInstanceDynamic.SetScalarParameterValue` _materialinstance_2 "DamageFactor" 0.0))
        (:`else`)))))

(event `self.PawnSensing.OnSeePawn`
  (params (Pawn :type "Pawn Object Reference"))
  ;[0.15 0.09132 0 0.5] 플레이어 시야 감지
  (switch `/Game/Blueprints/Game/Monster/EBearState` (`self.BearState`)
    (:`NewEnumerator0`
      (if (`self.ActorHasTag` Pawn "Player")
        (`BlackboardComponent.SetValueAsObject` (`AIController.Blackboard` (`AIBlueprintHelperLibrary.GetAIController` self)) (`self.TargetPlayerKey`) Pawn)
        (`self.SetState` "NewEnumerator1")))))

(event `OnAttackCheckStart`
  ;[0 1 0.468 0.5] 공격 충돌 판정 시작/종료
  (`PrimitiveComponent.SetCollisionEnabled` (`self.AttackCollision`) "QueryOnly"))

(event `OnAttackCheckEnd`
  ;[0 1 0.468 0.5] 공격 충돌 판정 시작/종료
  (`PrimitiveComponent.SetCollisionEnabled` (`self.AttackCollision`) "NoCollision"))

(event `self.AttackCollision.OnComponentBeginOverlap`
  (params (OverlappedComponent :type "PrimitiveComponent Object Reference") (OtherActor :type "Actor Object Reference") (OtherComp :type "PrimitiveComponent Object Reference") (OtherBodyIndex :type Integer) (bFromSweep :type Boolean) (SweepResult :type "HitResult Structure (by ref)"))
  (bind _monsterstat_attack (break `/Game/Blueprints/Game/Monster/Data/FMonsterData` (`/Game/Blueprints/Game/Monster/Data/BP_MonsterData.MonsterStat` (`/Game/Blueprints/Game/Component/BP_MonsterStat.MonsterData` (`self.MonsterStat`)))))
  ;[0.15 0.1032 0 0.5] 대미지 전달
  (if (`self.ActorHasTag` OtherActor "Player")
    (`GameplayStatics.ApplyDamage` OtherActor _monsterstat_attack (`AIBlueprintHelperLibrary.GetAIController` self) self)))

(fn `SetState`
  (params (NewState :type "/Game/Blueprints/Game/Monster/EBearState Enum" :default "NewEnumerator0"))
  (bind _charactermovement (`self.CharacterMovement`))
  (bind _monsterstat (`self.MonsterStat`))
  (bind (_monsterstat_attack _monsterstat_maxhp _monsterstat_walkspeed) (break `/Game/Blueprints/Game/Monster/Data/FMonsterData` (`/Game/Blueprints/Game/Monster/Data/BP_MonsterData.MonsterStat` (`/Game/Blueprints/Game/Component/BP_MonsterStat.MonsterData` _monsterstat))))
  (if (`|EnumInequality` (`self.BearState`) "NewEnumerator3")
    (bind _output_get (set `self.BearState` NewState))
    (`BlackboardComponent.SetValueAsEnum` (`AIController.Blackboard` (`AIBlueprintHelperLibrary.GetAIController` self)) (`self.StateKey`) _output_get)
    (switch `/Game/Blueprints/Game/Monster/EBearState` (`self.BearState`)
      (:`NewEnumerator0`
        (set `CharacterMovementComponent.MaxWalkSpeed` _monsterstat_walkspeed _charactermovement))
      (:`NewEnumerator1`
        (bind _output_get_2 (set `/Game/Blueprints/Game/Component/BP_MonsterStat.ChaseSpeed` (`self.Chase Speed`) _monsterstat))
        (set `CharacterMovementComponent.MaxWalkSpeed` _output_get_2 _charactermovement))
      (:`NewEnumerator2`
        (set `CharacterMovementComponent.MaxWalkSpeed` 0.0 _charactermovement :!label _label))
      (:`NewEnumerator3`
        (goto _label)))))

(fn `UserConstructionScript`)