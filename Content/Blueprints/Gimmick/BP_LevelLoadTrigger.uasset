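; Gimmick trigger actor that streams in its TargetLevel when an actor tagged Player overlaps it.
; The overlap runs a blocking soft-pointer level load set to be visible after load, then prints a Korean debug "loaded" message.
; After a short delay, it looks up the streaming level by TargetLevel's object name and sets ShouldBeVisible again.
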(event `self.ReceiveActorBeginOverlap`
  (params (OtherActor :type "Actor Object Reference"))
  (if (`self.ActorHasTag` OtherActor "Player")
    (`GameplayStatics.LoadStreamLevelBySoftObjectPtr` (`self.TargetLevel`) true true)
    (`KismetSystemLibrary.PrintString` "로드됨")
    (`KismetSystemLibrary.Delay` 3.0)
    (set `LevelStreaming.bShouldBeVisible` true (`GameplayStatics.GetStreamingLevel` (`KismetStringLibrary.Conv_StringToName` (`KismetSystemLibrary.GetObjectName` (`|ConvertAsset` (`self.TargetLevel`))))))))

(fn `UserConstructionScript`)