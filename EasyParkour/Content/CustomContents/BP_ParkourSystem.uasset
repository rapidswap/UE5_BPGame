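; Parkour component for BP_ThirdPersonCharacter that detects obstacles ahead and picks a move from wall height and horizontal speed.
; TriggerParkour chains stepped forward sphere traces, a line and sphere scan of wall face, top, far edge and landing, height measurement, then selection.
; Only One Hand Vault plays a montage, with Flying mode and capsule collision off until blend out; other moves just print.
; Tick updates the on-land check with a sphere trace.
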(event `TryVault`
  (params (VaultType :type "/Game/CustomContents/E_ValutType Enum" :default "NewEnumerator0"))
  (set `self.CanParkour` false)
  (bind _asbp_third_person_character (cast `/Game/ThirdPerson/Blueprints/BP_ThirdPersonCharacter` (`self.GetOwner`)))
  (`PrimitiveComponent.SetCollisionEnabled` (`Character.CapsuleComponent` _asbp_third_person_character) "NoCollision")
  (`CharacterMovementComponent.SetMovementMode` (`self.CharacterMovement`) "MOVE_Flying" 0)
  (switch `/Game/CustomContents/E_ValutType` VaultType
    (:`NewEnumerator0`
      (`|PlayMontage` (`self.PlayerMesh`) "/Game/Animations/OneHandVault_Montage.OneHandVault_Montage"
        (:`OnCompleted`
          (set `self.CanParkour` true))
        (:`OnBlendOut`
          (`PrimitiveComponent.SetCollisionEnabled` (`self.PlayerCapsule`) "QueryAndPhysics")
          (`CharacterMovementComponent.SetMovementMode` (`self.CharacterMovement`) "MOVE_Walking" 0))))))

(event `self.ReceiveTick`
  (params (DeltaSeconds :type "Float (single-precision)"))
  (bind _asbp_third_person_character (cast `/Game/ThirdPerson/Blueprints/BP_ThirdPersonCharacter` (`self.GetOwner`)))
  (bind _asbp_third_person_character_2 (cast `/Game/ThirdPerson/Blueprints/BP_ThirdPersonCharacter` (`self.GetOwner`)))
  (bind _returnvalue (`SceneComponent.K2_GetComponentLocation` (`Character.Mesh` _asbp_third_person_character_2)))
  (bind (_outhit _returnvalue_2) (`KismetSystemLibrary.SphereTraceSingle` :`Start` _returnvalue :`End` _returnvalue :`Radius` (`CapsuleComponent.GetUnscaledCapsuleRadius` (`Character.CapsuleComponent` _asbp_third_person_character)) :`TraceChannel` "TraceTypeQuery1" :`DrawDebugType` "ForOneFrame"))
  (set `self.IsOnLand` _returnvalue_2))

(fn `DetectWall`
  (returns (ReturnValue :type Boolean) (HitLocation :type "Vector Structure") (ReverseNormal :type "Rotator Structure"))
  (bind _returnvalue (`self.GetOwner`))
  (for _index (range 8)
    (bind _returnvalue_2 (`/Game/CustomContents/BP_Helper.MoveVectorUpward` (`/Game/CustomContents/BP_Helper.MoveVectorDownward` (`Actor.K2_GetActorLocation` _returnvalue) 60.0) (* _index 20.0)))
    (bind (_outhit _returnvalue_3) (`KismetSystemLibrary.SphereTraceSingle` :`Start` (`/Game/CustomContents/BP_Helper.MoveVectorBackward` _returnvalue_2 (`Actor.K2_GetActorRotation` _returnvalue) 30.0) :`End` (+ _returnvalue_2 (* (`Actor.GetActorForwardVector` _returnvalue) 200.0)) :`Radius` 10.0 :`TraceChannel` "TraceTypeQuery1" :`DrawDebugType` "ForOneFrame"))
    (if _returnvalue_3
      (`|ExecutionSequence`
        (:`then_0`
          (break))
        (:`then_1`
          (bind (_bblockinghit _binitialoverlap _time _distance _location _impactpoint _normal) (`GameplayStatics.BreakHitResult` _outhit))
          (return _bblockinghit _location (`/Game/CustomContents/BP_Helper.ReverseNormal` _normal)))))))

(fn `Initialize`
  (bind _returnvalue (message `/Game/CustomContents/Interfaces/BPI_Player.GetMesh` (`self.GetOwner`)))
  (set `self.PlayerMesh` _returnvalue)
  (bind _returnvalue_2 (message `/Game/CustomContents/Interfaces/BPI_Player.GetPlayerCapsule` (`self.GetOwner`)))
  (set `self.PlayerCapsule` _returnvalue_2)
  (bind _returnvalue_3 (message `/Game/CustomContents/Interfaces/BPI_Player.GetCharacterMovement` (`self.GetOwner`)))
  (set `self.CharacterMovement` _returnvalue_3))

(fn `MeasureWall`
  (if (and (`GameplayStatics.BreakHitResult` (`self.FacedWallHitResult`)) (`GameplayStatics.BreakHitResult` (`self.FirstTopHitResult`)))
    (bind _returnvalue (message `/Game/CustomContents/Interfaces/BPI_Player.GetMesh` (`self.GetOwner`)))
    (bind _output_get (set `self.WallHeight` (- (.z (`.ImpactPoint` (`GameplayStatics.BreakHitResult` (`self.FirstTopHitResult`)))) (.z (`SceneComponent.K2_GetComponentLocation` _returnvalue)))))
    (else
      (set `self.WallHeight` 0.0))))

(fn `ScanWall`
  (params (DetectLocation :type "Vector Structure") (ReversedNormal :type "Rotator Structure"))
  (locals (`ScanHitResultLocal ` :type "HitResult Structure"))
  (bind _reversed_normal (`self.Reversed Normal`))
  (bind (_bblockinghit _binitialoverlap _time _distance _location _impactpoint) (`GameplayStatics.BreakHitResult` (`self.LastTopHitResult`)))
  (bind (_bblockinghit_2 _binitialoverlap_2 _time_2 _distance_2 _location_2 _impactpoint_2 _normal) (`GameplayStatics.BreakHitResult` (`self.FacedWallHitResult`)))
  (for _index (range 30)
    (bind _returnvalue (`/Game/CustomContents/BP_Helper.MoveVectorDownward` (`/Game/CustomContents/BP_Helper.MoveVectorUpward` (`local.DetectLocation`) 300.0) (* _index 10)))
    (bind (_outhit _returnvalue_2) (`KismetSystemLibrary.LineTraceSingle` :`Start` (`/Game/CustomContents/BP_Helper.MoveVectorBackward` _returnvalue _reversed_normal 20.0) :`End` (`/Game/CustomContents/BP_Helper.MoveVectorForward` _returnvalue _reversed_normal 80.0) :`TraceChannel` "TraceTypeQuery1" :`DrawDebugType` "ForDuration"))
    (if _returnvalue_2
      (set `self.FacedWallHitResult` _outhit)
      (break)))
  (set `self.WallRotation` (`/Game/CustomContents/BP_Helper.ReverseNormal` _normal))
  (for _index_2 (range 10)
    (bind _returnvalue_3 (`/Game/CustomContents/BP_Helper.MoveVectorUpward` (`/Game/CustomContents/BP_Helper.MoveVectorForward` _location_2 (`self.WallRotation`) (* _index_2 20)) 10.0))
    (bind (_outhit_2 _returnvalue_4) (`KismetSystemLibrary.SphereTraceSingle` :`Start` _returnvalue_3 :`End` (`/Game/CustomContents/BP_Helper.MoveVectorDownward` _returnvalue_3 10.0) :`Radius` 5.0 :`TraceChannel` "TraceTypeQuery1" :`DrawDebugType` "ForDuration"))
    (if (== _index_2 0)
      (if _returnvalue_4
        (set `self.FirstTopHitResult` _outhit_2))
      (elif _returnvalue_4
        (set `self.LastTopHitResult` _outhit_2)
        (else
          (`|ExecutionSequence`
            (:`then_0`
              (break))
            (:`then_1`
              (bind (_outhit_3 _returnvalue_5) (`KismetSystemLibrary.SphereTraceSingle` :`Start` (`/Game/CustomContents/BP_Helper.MoveVectorForward` _impactpoint (`self.WallRotation`) 20.0) :`End` _impactpoint :`Radius` 10.0 :`TraceChannel` "TraceTypeQuery1" :`DrawDebugType` "ForDuration"))
              (if _returnvalue_5
                (bind _output_get (set `self.EndOfWallHitResult` _outhit_3))
                (bind _returnvalue_6 (`/Game/CustomContents/BP_Helper.MoveVectorForward` (`.ImpactPoint` (`GameplayStatics.BreakHitResult` _output_get)) (`self.WallRotation`) 60.0))
                (bind (_outhit_4 _returnvalue_7) (`KismetSystemLibrary.SphereTraceSingle` :`Start` _returnvalue_6 :`End` (`/Game/CustomContents/BP_Helper.MoveVectorDownward` _returnvalue_6 180.0) :`Radius` 10.0 :`TraceChannel` "TraceTypeQuery1" :`DrawDebugType` "ForDuration"))
                (if _returnvalue_7
                  (set `self.VaultLandingResult` _outhit_4))))))))))

(fn `TriggerParkour`
  (bind (_returnvalue _hitlocation _reversenormal) (`self.DetectWall`))
  (if _returnvalue
    (`self.ScanWall` _hitlocation _reversenormal)
    (`self.MeasureWall`)
    (`self.TryParkour`)))

(fn `TryParkour`
  (if (`GameplayStatics.BreakHitResult` (`self.FirstTopHitResult`))
    (if (`self.IsOnLand`)
      (if (<= (`self.WallHeight`) 300.0)
        (if (<= (`self.WallHeight`) 130.0)
          (if (not (`KismetMathLibrary.NearlyEqual_FloatFloat` (`KismetMathLibrary.VSizeXY` (`Actor.GetVelocity` (`self.GetOwner`))) 0.0 5.0))
            (if (> (`self.WallHeight`) 100.0)
              (`KismetSystemLibrary.PrintString` "Front Flip")
              (elif (> (`self.WallHeight`) 90.0)
                (`KismetSystemLibrary.PrintString` "Two Hand Vault")
                (else
                  (`KismetSystemLibrary.PrintString` "One Hand Vault")
                  (`self.TryVault` "NewEnumerator0"))))
            (else
              (`KismetSystemLibrary.PrintString` "Mantle")))
          (else
            (`KismetSystemLibrary.PrintString` "Climb")))
        (else
          (`KismetSystemLibrary.PrintString` "Wall Height is over 300"))))))